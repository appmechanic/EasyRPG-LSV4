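; BP_Notify_Footstep is an animation notify that triggers footstep actions on the animated character.
; When fired on a visible mesh, it finds the owner's BP_FootstepComponent and calls TryFootstep with the mesh, footstep type, foot side, foot index and sound flag.
; The footstep logic lives in that component, so owners without one are skipped.
; The notify's display name shows whether it is a left or right step.
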(fn ReceivedNotify
  (params (MeshComp :type Skeletal%20Mesh%20Component%20Object%20Reference) (Animation :type Anim%20Sequence%20Base%20Object%20Reference))
  (bind _returnvalue (Components|GetOwner MeshComp))
  (bind _returnvalue_2 (Actor|GetComponentbyClass _returnvalue "/Game/EasySurvivalRPG/Blueprints/Components/BP_FootstepComponent.BP_FootstepComponent_C"))
  ;[1 1 1] Execute footstep actions if character has footstep component.
  (LocalVariables|SetLocalMeshComponent MeshComp)
  (if (Rendering|IsVisible MeshComp)
    (Utilities|IsValid _returnvalue_2
      (:Is%20Valid
        (Default|TryFootstep _returnvalue_2 (LocalVariables|GetLocalMeshComponent) (Variables|Footstep|GetFootstepType) (Variables|Footstep|GetIsLeftFoot) (Variables|Footstep|GetFootIndex) (Variables|Footstep|GetPlaySound))
        (return true)))))

(fn GetNotifyName
  (return (Utilities|String|Append "Footstep_" (select (Variables|Footstep|GetIsLeftFoot) "Left" "Right"))))