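; Rideable horse character with camera-relative movement, jump, server-forwarded sprint and turn-in-place flags.
; Side trigger boxes offer interaction and pick the mount side; StartInteraction makes the player's controller possess the horse.
; A server/multicast toggle hides and attaches the player character while a stand-in Rider mesh plays mount animations.
; Dismount always exits right, then repossesses the character; much older mount/dismount logic remains disconnected.
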(event OnComponentBeginOverlap(L_Box)
  (params (OverlappedComponent :type Primitive%20Component%20Object%20Reference) (OtherActor :type Actor%20Object%20Reference) (OtherComp :type Primitive%20Component%20Object%20Reference) (OtherBodyIndex :type Integer) (bFromSweep :type Boolean) (SweepResult :type Hit%20Result%20Structure%20%28by%20ref%29))
  (Class|BPIPlayerCharacter|SetInteractable(Message) OtherActor self)
  (Variables|Default|SetRightMount? false))

(event OnComponentBeginOverlap(R_Box)
  (params (OverlappedComponent :type Primitive%20Component%20Object%20Reference) (OtherActor :type Actor%20Object%20Reference) (OtherComp :type Primitive%20Component%20Object%20Reference) (OtherBodyIndex :type Integer) (bFromSweep :type Boolean) (SweepResult :type Hit%20Result%20Structure%20%28by%20ref%29))
  (Class|BPIPlayerCharacter|SetInteractable(Message) OtherActor self)
  (Variables|Default|SetRightMount? true))

(event OnComponentEndOverlap(L_Box)
  (params (OverlappedComponent :type Primitive%20Component%20Object%20Reference) (OtherActor :type Actor%20Object%20Reference) (OtherComp :type Primitive%20Component%20Object%20Reference) (OtherBodyIndex :type Integer))
  (Class|BPIPlayerCharacter|SetInteractable(Message) OtherActor)
  (Variables|Default|SetRightMount? false))

(event OnComponentEndOverlap(R_Box)
  (params (OverlappedComponent :type Primitive%20Component%20Object%20Reference) (OtherActor :type Actor%20Object%20Reference) (OtherComp :type Primitive%20Component%20Object%20Reference) (OtherBodyIndex :type Integer))
  (Class|BPIPlayerCharacter|SetInteractable(Message) OtherActor)
  (Variables|Default|SetRightMount? false))

(event Custom|Mount
  (params (Character :type ALS%20Anim%20Man%20ESRPG%20Player%20BP%20Object%20Reference) (Right? :type Boolean)))

(event Custom|Server_Mount
  (params (Character :type ALS%20Anim%20Man%20ESRPG%20Player%20BP%20Object%20Reference) (Right? :type Boolean) (Rider :type Skeletal%20Mesh%20Component%20Object%20Reference) (Controller :type Player%20Controller%20Object%20Reference))
  ;[1 1 1] Mount
)

(event Custom|Multicast_MountHorse
  (params (RiderCharacter :type Character%20Object%20Reference)))

(event Custom|Server_MountHorse
  (params (RiderCharacter :type Character%20Object%20Reference))
  (CallFunction|MulticastMountHorse RiderCharacter))

(event Custom|ServerToggleRider
  (params (Enable :type Boolean))
  (CallFunction|MulticastToggleRider Enable))

(event Custom|MulticastToggleRider
  (params (Enable :type Boolean))
  (bind _returnvalue (Pawn|GetController))
  (bind _returnvalue_2 (Game|GetPlayerController 0))
  (bind _self self)
  (bind _rider (Variables|Default|GetRider))
  (bind _rider_2 (Variables|Default|GetRider))
  (bind _rider_3 (Variables|Default|GetRider))
  (bind _ridercharacter (Variables|Default|GetRiderCharacter))
  (bind _ridercharacter_2 (Variables|Default|GetRiderCharacter))
  (if Enable
    (Transformation|AttachComponentToComponent _ridercharacter_2 (Variables|Character|GetMesh) "MountPoint" "KeepRelative" "KeepRelative" "KeepRelative" true)
    (Collision|SetActorEnableCollision _ridercharacter_2 false)
    (Rendering|SetActorHiddenInGame _ridercharacter_2 true)
    (Rendering|SetVisibility (Variables|Default|GetRider) true false)
    (if (Variables|Default|GetRightMount?)
      (Transformation|SetRelativeTransform _rider_2 (Math|Transform|MakeTransform "0.000597,14.956697,-150.000000" "0, 0,-7.356973" "1,1,1") true false)
      (Components|Animation|PlayAnimation _rider_2 "/Game/HorseAnimsetPro/Animations/Rider_Mannequin/Rider_Mount_Right.Rider_Mount_Right" false)
      (else
        (Transformation|SetRelativeTransform _rider_3 (Math|Transform|MakeTransform "0.000597,14.956697,-150.000000" "0, 0,-7.356973" "1,1,1") true false)
        (Components|Animation|PlayAnimation _rider_3 "/Game/HorseAnimsetPro/Animations/Rider_Mannequin/Rider_Mount_Left.Rider_Mount_Left" false)))
    (Input|DisableInput _self _returnvalue_2)
    (Utilities|FlowControl|Delay 1.75)
    (Input|EnableInput _self _returnvalue_2)
    (else
      (Utilities|IsValid _ridercharacter
        (:Is%20Valid
          (Input|DisableInput self (Game|GetPlayerController 0))
          (Transformation|DetachFromActor _ridercharacter "KeepRelative" "KeepRelative" "KeepRelative")
          (Collision|SetActorEnableCollision _ridercharacter true)
          (Transformation|SetRelativeTransform _rider (Math|Transform|MakeTransform "0.000597,14.956697,-150.000000" "0, 0,-7.356973" "1,1,1") true false)
          (Components|Animation|PlayAnimation _rider "/Game/HorseAnimsetPro/Animations/Rider_Mannequin_V2/Rider_Dismount_Right_v2.Rider_Dismount_Right_v2" false)
          (Transformation|SetWorldLocation (Variables|/Script/Engine.Actor|GetRootComponent _ridercharacter) (Transformation|GetWorldLocation (Variables|Default|GetRightDismount)) false true)
          (Utilities|FlowControl|Delay 1.75)
          (Rendering|SetVisibility (Variables|Default|GetRider) false false)
          (Rendering|SetActorHiddenInGame _ridercharacter false)
          (Utilities|FlowControl|Delay 1.0)
          ;[1 1 1] Mount
          (Utilities|IsValid _returnvalue
            (:Is%20Valid
              (Pawn|Possess _returnvalue _ridercharacter))))))))

(event Custom|MulticastMount
  (params (Character :type ALS%20Anim%20Man%20ESRPG%20Player%20BP%20Object%20Reference) (Right? :type Boolean) (Rider :type Skeletal%20Mesh%20Component%20Object%20Reference) (Controller :type Player%20Controller%20Object%20Reference))
  ;[1 1 1] Mount
)

(event Custom|Server_Dismount
  (params (Character :type ALS%20Anim%20Man%20ESRPG%20Player%20BP%20Object%20Reference) (Rider :type Skeletal%20Mesh%20Component%20Object%20Reference) (Controller :type Player%20Controller%20Object%20Reference))
  ;[1 1 1] Dismount
)

(event Custom|MulticastDismount
  (params (Character :type ALS%20Anim%20Man%20ESRPG%20Player%20BP%20Object%20Reference) (Rider :type Skeletal%20Mesh%20Component%20Object%20Reference) (Controller :type Player%20Controller%20Object%20Reference)))

(event Custom|ClientDismount
  ;[1 1 1] Dismount
)

(event Custom|ClientMount
  (params (Character :type ALS%20Anim%20Man%20ESRPG%20Player%20BP%20Object%20Reference) (Right? :type Boolean)))

(event Custom|SprintServer
  (params (Speed :type Float%20%28single-precision%29))
  ;[1 1 1] Input Action
  (Variables|/Script/Engine.CharacterMovementComponent|SetMaxWalkSpeed (Variables|Character|GetCharacterMovement) Speed))

(event EventBeginPlay)

(event Collision|EventActorBeginOverlap
  (params (OtherActor :type Actor%20Object%20Reference)))

(event EventTick
  (params (DeltaSeconds :type Float%20%28single-precision%29)))

(event EventTryInteractBPI
  (params (Release :type Boolean) (PlayerController :type Player%20Controller%20Object%20Reference)))

(event EventStartInteraction
  (params (Rider :type Character%20Object%20Reference))
  (bind _output_get (Variables|Default|SetRiderCharacter Rider))
  (bind _controller (Class|BPIPlayerCharacter|GetCharacterControllerReference(Message) _output_get))
  (Utilities|IsValid _controller
    (:Is%20Valid
      (Pawn|Possess _controller self)
      (Networking|SwitchHasAuthority
        (:Authority
          (CallFunction|MulticastToggleRider true))
        (:Remote
          (CallFunction|ServerToggleRider true))))))

(event EventStartInteraction
  (params (InteractingCharacter :type Character%20Object%20Reference)))

(event Input|ActionEvents|InputActionJump
  (params (Key :type Key%20Structure :default "None"))
  ;[1 1 1] Input Action
  (:Pressed
    (Character|Jump))
  (:Released
    (Character|StopJumping)))

(event Input|ActionEvents|InputActionHorseSprint
  (params (Key :type Key%20Structure :default "None"))
  (bind _charactermovement (Variables|Character|GetCharacterMovement))
  ;[1 1 1] Input Action
  (:Pressed
    (bind _output_get (Variables|/Script/Engine.CharacterMovementComponent|SetMaxWalkSpeed _charactermovement 6e+02))
    (CallFunction|SprintServer _output_get))
  (:Released
    (bind _output_get_2 (Variables|/Script/Engine.CharacterMovementComponent|SetMaxWalkSpeed _charactermovement 3e+02))
    (CallFunction|SprintServer _output_get_2)))

(event Input|ActionEvents|InputActionHorseMount/Dismount
  (params (Key :type Key%20Structure :default "None"))
  (:Pressed
    (Networking|SwitchHasAuthority
      (:Authority
        (CallFunction|MulticastToggleRider false))
      (:Remote
        (CallFunction|ServerToggleRider false)))))

(event Input|AxisEvents|InputAxisMoveRight
  (params (AxisValue :type Float%20%28single-precision%29))
  ;[1 1 1] Input Action
  (Pawn|Input|AddMovementInput (Math|Vector|GetRightVector (Math|Rotator|MakeRotator 0.0 0.0 (.Yaw (Math|Rotator|BreakRotator (Pawn|GetControlRotation :!class /Script/Engine.Pawn))))) AxisValue false))

(event Input|AxisEvents|InputAxisMoveForward
  (params (AxisValue :type Float%20%28single-precision%29))
  ;[1 1 1] Input Action
  (Pawn|Input|AddMovementInput (Math|Vector|GetForwardVector (Math|Rotator|MakeRotator 0.0 0.0 (.Yaw (Math|Rotator|BreakRotator (Pawn|GetControlRotation :!class /Script/Engine.Pawn))))) AxisValue false))

(event Input|AxisEvents|InputAxisTurn
  (params (AxisValue :type Float%20%28single-precision%29))
  (bind _returnvalue (Input|AxisValues|GetTurn))
  ;[1 1 1] Input Action
  (Pawn|Input|AddControllerYawInput AxisValue)
  (if (== (Math|Vector|VectorLength (Transformation|GetVelocity)) 0.0)
    (Utilities|FlowControl|Sequence
      (:then_0
        (if (> _returnvalue 0.2)
          (Variables|Default|SetTurnRight? true)
          (else
            (Variables|Default|SetTurnRight? false))))
      (:then_1
        (if (< _returnvalue -0.2)
          (Variables|Default|SetTurnLeft? true)
          (else
            (Variables|Default|SetTurnLeft? false)))))
    (else
      (Variables|Default|SetTurnLeft? false)
      (Variables|Default|SetTurnRight? false))))

(event Input|AxisEvents|InputAxisLookUp
  (params (AxisValue :type Float%20%28single-precision%29))
  ;[1 1 1] Input Action
  (Pawn|Input|AddControllerPitchInput AxisValue))

(event Input|KeyboardEvents|F
  (params (Key :type Key%20Structure :default "None"))
  ;[1 1 1] Dismount
)

(fn ConstructionScript)

(fn CheckCanInteractBPI
  (params (PlayerController :type Player%20Controller%20Object%20Reference))
  (return false))

(fn GetInteractionObjectNameBPI
  (return ""))

(fn GetInteractionTextBPI
  (params (PlayerController :type Player%20Controller%20Object%20Reference))
  (return ""))

(fn IsTurnedonBPI
  (return false))